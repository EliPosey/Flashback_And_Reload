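; BASIC_GAMESTATE is a Game State Blueprint meant to gather player controllers and spawn a possessed character for each, currently dormant.
; GetAllPlayerControllers casts each PlayerArray entry's owner to Basic_PLAYCON and stores it in CharacterControllerArray.
; SpawnCharacters spawns a Temp_Char per controller at indexed locations, possesses it, then records a BASIC_CHARACTER reference from an unexecuted cast.
; BeginPlay is empty, and the delayed chain calling both routines is disconnected.
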(event Custom|Spawn%20Characters
  (bind _character_controller_array (Variables|Default|GetCharacter%20Controller%20Array))
  (bind (_2d_character_array _playcon_refs) (Utilities|Struct|BreakChar_Con_Association _character_controller_array))
  (bind (_array_element _array_index) (Utilities|Array|ForEachLoopwithBreak _playcon_refs)
    (:LoopBody
      (bind _returnvalue (Game|SpawnActorfromClass "/Game/Flashback_And_Reload/Blueprints/Temp_Char.Temp_Char_C" (Math|Transform|MakeTransform (Utilities|Array|Get(acopy) (Variables|Default|GetLocation) _array_index)) false 0))
      (bind _astemp_char (Utilities|Casting|CastToTemp_Char _returnvalue)
        (:then
          (Pawn|Possess _array_element _astemp_char)
          (Utilities|Array|Add (Utilities|Struct|BreakCharacterArray (Utilities|Array|Get(acopy) _2d_character_array _array_index)) (stale _asbasic_character)))
        (:CastFailed
          (Development|PrintString "Failed"))))))

(event EventBeginPlay)

(fn ConstructionScript)

(fn GetAllPlayerControllers
  (for _array_element (Variables|Default|GetPlayerArray)
    (bind _asbasic_playcon (Utilities|Casting|CastToBasic_PLAYCON (Components|GetOwner _array_element))
      (:then
        (Development|PrintString "YES")
        (Utilities|Array|Add (.PlayCON_refs (Utilities|Struct|BreakChar_Con_Association (Variables|Default|GetCharacter%20Controller%20Array))) _asbasic_playcon))
      (:CastFailed
        (Development|PrintString "Hello")))))