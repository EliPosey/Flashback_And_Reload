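; Spawn manager for a flashback mechanic that adds unpossessed copies of the player character, each given a recording of the player's actions.
; On BeginPlay it spawns a FAR_Character at a fixed point and possesses it.
; A Delay on Tick periodically stores the first character's ActionRecording, then spawns up to five unpossessed characters at that point, assigning each the recording at PossessionIndex.
; SpawnCharacter handles both cases and tracks every character in an array.
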(event EventBeginPlay
  (CallFunction|SpawnCharacter true "-1500.000000,-65.000000,20.000000"))

(event EventTick
  (params (DeltaSeconds :type Float%20%28single-precision%29))
  (Utilities|FlowControl|Delay 5.0)
  (Utilities|Array|Add (Variables|Default|GetRecordings) (Variables|/Game/Flashback_And_Reload/Blueprints/FAR_Character.FAR_Character_C|GetAction%20Recording (Utilities|Array|Get(acopy) (Variables|Default|GetCharacters))))
  (Utilities|FlowControl|DoN 5
    (:Exit
      (bind _spawned_character (CallFunction|SpawnCharacter false "-1500.000000,-65.000000,20.000000"))
      (Variables|/Game/Flashback_And_Reload/Blueprints/FAR_Character.FAR_Character_C|SetAction%20Recording _spawned_character (Utilities|Array|Get(acopy) (Variables|Default|GetRecordings) (Variables|Default|GetPossession%20Index))))))

(fn ConstructionScript)

(fn SpawnCharacter
  (params (Give%20Possession? :type Boolean) (Spawn%20Location :type Vector))
  (bind _returnvalue (Game|SpawnActorfromClass "/Game/Flashback_And_Reload/Blueprints/FAR_Character.FAR_Character_C" (Math|Transform|MakeTransform Spawn%20Location) true 0))
  (bind _asfar_character (Utilities|Casting|CastToFAR_Character _returnvalue))
  (if Give%20Possession?
    (Utilities|Array|Add (Variables|Default|GetCharacters) _asfar_character)
    (if (Utilities|IsValid _asfar_character)
      (Pawn|Possess (Game|GetPlayerController (Variables|Default|GetController%20Association)) _asfar_character)
      (return _asfar_character)
      (else
        (Development|PrintString "Nec Char is not valid")))
    (elif (Utilities|IsValid _asfar_character)
      (Utilities|Array|Add (Variables|Default|GetCharacters) _asfar_character)
      (return _asfar_character)
      (else
        (Development|PrintString "Nec Char is not valid")))))