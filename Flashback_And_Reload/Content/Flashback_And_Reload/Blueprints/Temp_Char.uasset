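; Temporary player character for Flashback_And_Reload with movement, shooting, health and a possession flag.
; A custom event spawns an automatic Weapon_Template in front of the character and attaches it; fire input starts and halts it.
; All damage reduces HitPoints, but only Prototype_Projectile hits can destroy the character and weapon.
; Flashlight input calls a toggle; reload casts an unconnected object to BASIC_CHARACTER, so it never reaches the weapon.
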(event Custom|Move%20Side%20to%20SIde
  (params (Axis :type Float%20%28single-precision%29 :default 0.0))
  (Pawn|Input|AddMovementInput (Math|Vector|GetRightVector (Pawn|GetControlRotation :!class /Script/Engine.Pawn)) Axis false))

(event Custom|Stop_Fire
  (Default|HaultFire (Variables|Default|GetWeapon)))

(event Custom|Fire
  (Default|FireWeapon (Variables|Default|GetWeapon)))

(event Custom|add%20weapon%20to%20character
  (bind _returnvalue (Transformation|GetActorRotation))
  ;[1 0.9766 0] ADD WEAPON TO CHARACTER
  (bind _returnvalue_2 (Game|SpawnActorfromClass "/Game/Flashback_And_Reload/Weapons/Weapon_Template.Weapon_Template_C" (Math|Transform|MakeTransform (+ (Transformation|GetActorLocation) (* (Math|Vector|GetForwardVector _returnvalue) 6e+01)) _returnvalue "1.000000,1.000000,1.000000") true 0 true 1.2e+03 0.05 100 1000 1.5 1))
  (bind _asweapon_template (Utilities|Casting|CastToWeapon_Template _returnvalue_2)
    (:then
      (Class|Actor|AttachRootComponenttoActor _asweapon_template self "None" "SnapToTarget" true)
      (Variables|Default|SetWeapon _asweapon_template))
    (:CastFailed
      (Development|PrintString "Cast To Weapon_Template in FAR_Character has Failed"))))

(event Custom|Move%20Forward/Backwards
  (params (Axis :type Float%20%28single-precision%29))
  (Pawn|Input|AddMovementInput (Math|Vector|GetForwardVector (Pawn|GetControlRotation :!class /Script/Engine.Pawn)) Axis false))

(event EventAnyDamage
  (params (Damage :type Float%20%28single-precision%29) (DamageType :type Damage%20Type%20Object%20Reference) (InstigatedBy :type Controller%20Object%20Reference) (DamageCauser :type Actor%20Object%20Reference))
  ;[0 0.9234 1] Apply Damage to Character
  (Variables|Default|SetHit%20Points (- (Variables|Default|GetHit%20Points) Damage))
  (Utilities|Casting|CastToPrototype_Projectile DamageCauser)
  (if (<= (Variables|Default|GetHit%20Points) 0.0)
    (Actor|DestroyActor (Variables|Default|GetWeapon))
    (Actor|DestroyActor)))

(event EventPossessed
  (params (NewController :type Controller%20Object%20Reference))
  ;[0 0 0] If Unpossessed set True. If Possessed set False (FOR NOW)
  (Development|PrintString "Possessed")
  (Variables|Default|SetIsPossessed? true))

(event EventUnpossessed
  (params (OldController :type Controller%20Object%20Reference))
  ;[0 0 0] If Unpossessed set True. If Possessed set False (FOR NOW)
  (Development|PrintString "Unpossessed")
  (Variables|Default|SetIsPossessed? false))

(event Input|ActionEvents|InputActionFlashLight
  (:Pressed
    (CallFunction|ToggleFlashlight)))

(event Input|ActionEvents|InputActionFire
  (:Pressed
    (CallFunction|Fire))
  (:Released
    (CallFunction|StopFire)))

(event Input|ActionEvents|InputActionReload
  (:Pressed
    (bind _asbasic_character (Utilities|Casting|CastToBASIC_CHARACTER))
    (Default|ManualReload (Variables|/Game/Flashback_And_Reload/Player/BASIC_CHARACTER.BASIC_CHARACTER_C|GetWeapon _asbasic_character))))

(event Input|AxisEvents|InputAxisMoveForward
  (params (AxisValue :type Float%20%28single-precision%29))
  (CallFunction|MoveForward/Backwards AxisValue))

(event Input|AxisEvents|InputAxisMoveSidetoSide
  (params (AxisValue :type Float%20%28single-precision%29))
  (CallFunction|MoveSidetoSIde AxisValue))

(fn ConstructionScript)