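; Player controller for the Flashback And Reload game that drives the FAR_Character pawn and quits the game on Escape.
; On BeginPlay for a local player it switches to fullscreen, caches the character, enables its recording state and temporarily adds a weapon.
; Inputs move the pawn relative to control rotation and forward fire, reload and flashlight actions to the character or its weapon.
; Tick yaws the pawn toward the deprojected mouse cursor position.
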(event EventTick
  (params (DeltaSeconds :type Float%20%28single-precision%29))
  (bind (_locationx _locationy) (Game|Player|GetMousePosition))
  (bind _returnvalue (Pawn|GetControlledPawn))
  (Utilities|FlowControl|Sequence
    (:then_0
      ;[0.07124 1 0] Rotation
      (Transformation|SetActorRotation _returnvalue (Class|KismetMathLibrary|MakeRot 0.0 (.Yaw (Class|KismetMathLibrary|BreakRot (Math|Rotator|FindLookatRotation (Transformation|GetActorLocation _returnvalue) (.WorldLocation (Class|PlayerController|DeprojectScreenPositiontoWorld _locationx _locationy))))) 0.0)))))

(event EventBeginPlay
  ;[1 1 1] Make game Fullscreen Mode
  (if (and (Pawn|IsLocalPlayerController) (not (Networking|IsDedicatedServer)))
    (Development|ExecuteConsoleCommand "FULLSCREEN")
    ;[0.1624 0.4138 0.495] Setting Controlled Character
    (bind _asfar_character (Utilities|Casting|CastToFAR_Character (Pawn|GetControlledPawn))
      (:then
        (Variables|Default|SetControlled%20Character _asfar_character)
        (Variables|/Game/Flashback_And_Reload/Blueprints/FAR_Character.FAR_Character_C|SetRecording%20State _asfar_character true)
        ;[1 1 1] TEMPORARY : adds a weapon to character
        (Default|AddWeapontoCharacter (Variables|Default|GetControlled%20Character)))
      (:CastFailed
        (Development|PrintString "Cast To FAR_Character in FAR_PlayerController has Failed")))))

(event Input|ActionEvents|InputActionFlashLight
  (:Pressed
    (Default|ToggleFlashlight (Variables|Default|GetControlled%20Character))))

(event Input|ActionEvents|InputActionFire
  (bind _controlled_character (Variables|Default|GetControlled%20Character))
  (bind _weapon (Variables|/Game/Flashback_And_Reload/Blueprints/FAR_Character.FAR_Character_C|GetWeapon _controlled_character))
  (:Pressed
    (Default|FireWeapon _weapon))
  (:Released
    (Default|HaultFire _weapon)))

(event Input|ActionEvents|InputActionReload
  (:Pressed
    (Default|ManualReload (Variables|/Game/Flashback_And_Reload/Blueprints/FAR_Character.FAR_Character_C|GetWeapon (Variables|Default|GetControlled%20Character)))))

(event Input|AxisEvents|InputAxisMoveForward
  (params (AxisValue :type Float%20%28single-precision%29))
  ;[0 1 0.05458] Character Movement
  (Pawn|Input|AddMovementInput (Pawn|GetControlledPawn) (Math|Vector|GetForwardVector (Pawn|GetControlRotation :!class /Script/Engine.Controller)) AxisValue false))

(event Input|AxisEvents|InputAxisMoveSidetoSide
  (params (AxisValue :type Float%20%28single-precision%29))
  ;[0 1 0.05458] Character Movement
  (Pawn|Input|AddMovementInput (Pawn|GetControlledPawn) (Math|Vector|GetRightVector (Pawn|GetControlRotation :!class /Script/Engine.Controller)) AxisValue false))

(event Input|KeyboardEvents|Escape
  (:Pressed
    ;[1 1 1] Quit Game
    (Game|QuitGame 0 "Quit")))

(fn ConstructionScript)