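; FAR_Character is a character that records the player's actions while possessed and replays them once unpossessed.
; At BeginPlay it spawns an Action_Recording actor, whose per-tick arrays store transform, reload, flashlight and interaction states while RecordingState is on.
; Playback steps an index through those arrays each tick; weapon fire always records false and interaction replay is empty.
; A separate event spawns and attaches a Weapon_Template as its weapon.
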(event Custom|add%20weapon%20to%20character
  (bind _returnvalue (Transformation|GetActorRotation))
  ;[1 1 1] ADD WEAPON TO CHARACTER
  (bind _returnvalue_2 (Game|SpawnActorfromClass "/Game/Flashback_And_Reload/Weapons/Weapon_Template.Weapon_Template_C" (Math|Transform|MakeTransform (+ (Transformation|GetActorLocation) (* (Math|Vector|GetForwardVector _returnvalue) 6e+01)) _returnvalue "1.000000,1.000000,1.000000") true 0 false 1.2e+03 0.0 2 5 1.5 1))
  (bind _asweapon_template (Utilities|Casting|CastToWeapon_Template _returnvalue_2)
    (:then
      (Class|Actor|AttachRootComponenttoActor _asweapon_template self "None" "SnapToTarget" true)
      (Variables|Default|SetWeapon _asweapon_template))
    (:CastFailed
      (Development|PrintString "Cast To Weapon_Template in FAR_Character has Failed"))))

(event Custom|Apply%20Actions
  ;[1 0 1] Apply Movement and Rotation
  (Development|PrintString "Applying")
  (Transformation|SetActorTransform (Utilities|Array|Get(acopy) (Variables|/Game/Flashback_And_Reload/Blueprints/Action_Recording.Action_Recording_C|GetCharacter%20Transform (Variables|RecordingInfo|GetAction%20Recording)) (Variables|Counts|GetNon_Specific%20Count)) true)
  (Utilities|FlowControl|Sequence
    (:then_0
      ;[1 0 0] "Reload Weapon"
      (if (Utilities|Array|Get(acopy) (Variables|/Game/Flashback_And_Reload/Blueprints/Action_Recording.Action_Recording_C|GetReload? (Variables|RecordingInfo|GetAction%20Recording)) (Variables|Counts|GetNon_Specific%20Count))
        (Default|ReloadWeapon (Variables|Default|GetWeapon))))
    (:then_1
      ;[0 0 1] Fire Weapon and Apply Spread Value
      (if (Utilities|Array|Get(acopy) (Variables|/Game/Flashback_And_Reload/Blueprints/Action_Recording.Action_Recording_C|GetWeapon%20Fire? (Variables|RecordingInfo|GetAction%20Recording)) (Variables|Counts|GetNon_Specific%20Count))
        (Default|FireWeapon (Variables|Default|GetWeapon))
        (Variables|Counts|SetSpread%20Value%20Count (+ (Variables|Counts|GetSpread%20Value%20Count) 1))))
    (:then_2
      ;[0 1 0] Toggle Flashlight
      (if (Utilities|Array|Get(acopy) (Variables|/Game/Flashback_And_Reload/Blueprints/Action_Recording.Action_Recording_C|GetFlashlight%20Toggle? (Variables|RecordingInfo|GetAction%20Recording)) (Variables|Counts|GetNon_Specific%20Count))
        (CallFunction|ToggleFlashlight)))
    (:then_3
      ;[1 1 0] Interact
      (if (Utilities|Array|Get(acopy) (Variables|/Game/Flashback_And_Reload/Blueprints/Action_Recording.Action_Recording_C|GetInteraction? (Variables|RecordingInfo|GetAction%20Recording)) (Variables|Counts|GetNon_Specific%20Count))
        _))
    (:then_4
      (Variables|Counts|SetNon_Specific%20Count (+ (Variables|Counts|GetNon_Specific%20Count) 1)))))

(event EventTick
  (params (DeltaSeconds :type Float%20%28single-precision%29))
  ;[1 0 0] Record Actions / Apply Actions
  (if (Variables|RecordingInfo|GetIs%20Possessed?)
    (CallFunction|RecordActions)
    (else
      (CallFunction|ApplyActions))))

(event EventBeginPlay
  (bind _returnvalue (Game|SpawnActorfromClass "/Game/Flashback_And_Reload/Blueprints/Action_Recording.Action_Recording_C" (Transformation|GetActorTransform) true 0))
  (bind _asaction_recording (Utilities|Casting|CastToAction_Recording _returnvalue))
  (Variables|RecordingInfo|SetAction%20Recording _asaction_recording))

(event EventPossessed
  (params (NewController :type Controller%20Object%20Reference))
  ;[0 0 0] If Unpossessed set True. If Possessed set False (FOR NOW)
  (Development|PrintString "Possessed")
  (Variables|RecordingInfo|SetIs%20Possessed? true))

(event EventUnpossessed
  (params (OldController :type Controller%20Object%20Reference))
  ;[0 0 0] If Unpossessed set True. If Possessed set False (FOR NOW)
  (Development|PrintString "Unpossessed")
  (Variables|RecordingInfo|SetIs%20Possessed? false))

(fn ConstructionScript)

(fn RecordActions
  (bind _weapon (Variables|Default|GetWeapon))
  (bind _action_recording (Variables|RecordingInfo|GetAction%20Recording))
  (if (Variables|RecordingInfo|GetRecording%20State)
    (if (Utilities|IsValid _action_recording)
      (Utilities|Array|Add (Variables|/Game/Flashback_And_Reload/Blueprints/Action_Recording.Action_Recording_C|GetCharacter%20Transform _action_recording) (Transformation|GetActorTransform))
      (Utilities|Array|Add (Variables|/Game/Flashback_And_Reload/Blueprints/Action_Recording.Action_Recording_C|GetReload? _action_recording) (Variables|/Game/Flashback_And_Reload/Weapons/Weapon_Template.Weapon_Template_C|GetReload%20State _weapon))
      (Variables|/Game/Flashback_And_Reload/Weapons/Weapon_Template.Weapon_Template_C|SetReload%20State _weapon false)
      (Utilities|Array|Add (Variables|/Game/Flashback_And_Reload/Blueprints/Action_Recording.Action_Recording_C|GetWeapon%20Fire? _action_recording) false)
      (if (Variables|/Game/Flashback_And_Reload/Weapons/Weapon_Template.Weapon_Template_C|GetFire%20Weapon%20State _weapon)
        (Utilities|Array|Add (Variables|/Game/Flashback_And_Reload/Blueprints/Action_Recording.Action_Recording_C|GetSpread%20Value _action_recording) (Variables|RecordingInfo|GetCurrent%20Spread%20Value)))
      (Utilities|Array|Add (Variables|/Game/Flashback_And_Reload/Blueprints/Action_Recording.Action_Recording_C|GetFlashlight%20Toggle? _action_recording) (Variables|RecordingInfo|GetCurrent%20Flashlight%20State))
      (Variables|RecordingInfo|SetCurrent%20Flashlight%20State false)
      (Utilities|Array|Add (Variables|/Game/Flashback_And_Reload/Blueprints/Action_Recording.Action_Recording_C|GetInteraction? _action_recording) (Variables|RecordingInfo|GetCurrent%20Interaction%20State))
      (else
        (Development|PrintString "Action Recording Invalid")))))

(fn ToggleFlashlight
  (Variables|RecordingInfo|SetCurrent%20Flashlight%20State true)
  ;[1 1 1] Toggle Flashlight
  (Rendering|ToggleVisibility (Variables|Default|GetFlashLight) false))