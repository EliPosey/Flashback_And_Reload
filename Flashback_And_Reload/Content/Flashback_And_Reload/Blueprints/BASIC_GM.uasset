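; Game mode that runs a round-based match in which players' recorded past runs return as duplicate characters.
; On login it numbers players and stores controllers, later spawning characters at matching spawn points.
; A Tick-driven state machine, gated open after BeginPlay, uses timelines for shop, countdown and round phases.
; Preparing spawns input-blocked players and recording-fed duplicates, countdown unblocks input, and round end kills all characters and repeats while rounds remain.
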(event Custom|Reset%20Timers
  (Utilities|FlowControl|Sequence
    (:then_0
      (bind _shop_timer (Timeline|Shop%20Timer Stop)
        (:Update
          (bind _output_get (Variables|RoundInfo|SetTime _shop_timer))
          (Development|PrintString (Utilities|String|ToString(Float) _output_get)))
        (:Finished
          (Variables|RoundInfo|SetRound%20State "NewEnumerator2")
          (CallFunction|ResetTimers))))
    (:then_1
      (Timeline|Shop%20Timer SetNewTime))
    (:then_2
      (bind _countdown (Timeline|Countdown%20Timer Stop)
        (:Update
          (bind _output_get_2 (Variables|RoundInfo|SetTime _countdown))
          (Development|PrintString (Utilities|String|ToString(Float) _output_get_2) true true "(R=0.000000,G=1.000000,B=0.095898,A=1.000000)"))
        (:Finished
          (CallFunction|MassInputUn/BLock false)
          (Variables|RoundInfo|SetRound%20State "NewEnumerator3")
          (CallFunction|ResetTimers))))
    (:then_3
      (Timeline|Countdown%20Timer SetNewTime))
    (:then_4
      (bind _round_time (Timeline|Round%20Timer Stop)
        (:Update
          (bind _output_get_3 (Variables|RoundInfo|SetTime _round_time)))
        (:Finished
          (Variables|RoundInfo|SetRound%20Over true)
          (Variables|RoundInfo|SetRound%20State "NewEnumerator4")
          (CallFunction|ResetTimers))))
    (:then_5
      (Timeline|Round%20Timer SetNewTime))))

(event Custom|Spawn%20Duplicate
  ;[0 0 0] Spawn Duplicate
  (bind _array_element (Utilities|Array|ForEachLoopwithBreak (Variables|Default|GetController%20Array))
    (:LoopBody
      (bind _asplayer_state_main (Utilities|Casting|CastToPlayerState_Main (Variables|/Script/Engine.Controller|GetPlayerState _array_element))
        (:then
          (bind _array_element_2 (Utilities|Array|ForEachLoopwithBreak (Variables|/Game/Flashback_And_Reload/Player/PlayerState_Main.PlayerState_Main_C|GetArray%20of%20recordings _asplayer_state_main))
            (:LoopBody
              (bind _returnvalue (Game|SpawnActorfromClass "/Game/Flashback_And_Reload/Player/Character_Main.Character_Main_C" (Utilities|Array|Get(acopy) (.Transform (Utilities|Struct|BreakActionRecord _array_element_2))) false 0 "NewEnumerator1" 0))
              (Variables|/Game/Flashback_And_Reload/Player/Character_Main.Character_Main_C|Setrecord _returnvalue _array_element_2)
              (Utilities|Array|AddUnique (Variables|/Game/Flashback_And_Reload/Player/PlayerState_Main.PlayerState_Main_C|GetCharacter%20References _asplayer_state_main) _returnvalue))))
        (:CastFailed
          (Development|PrintString "Cast to PlayerState_Main in BASIC_GM in Spawn Duplicates has FAILED"))))))

(event Custom|State%20Event
  (switch Utilities|FlowControl|Switch|SwitchonRoundState (Variables|RoundInfo|GetRound%20State)
    (:NewEnumerator0
      (CallFunction|ClearAllCharacterArrays)
      (CallFunction|SpawnCharacters)
      (CallFunction|SpawnDuplicate)
      (Variables|RoundInfo|SetRound%20State "NewEnumerator2"))
    (:NewEnumerator1
      (bind _shop_timer (Timeline|Shop%20Timer Play)
        (:Update
          (bind _output_get (Variables|RoundInfo|SetTime _shop_timer))
          (Development|PrintString (Utilities|String|ToString(Float) _output_get)))
        (:Finished
          (Variables|RoundInfo|SetRound%20State "NewEnumerator2")
          (CallFunction|ResetTimers))))
    (:NewEnumerator2
      (bind _countdown (Timeline|Countdown%20Timer Play)
        (:Update
          (bind _output_get_2 (Variables|RoundInfo|SetTime _countdown))
          (Development|PrintString (Utilities|String|ToString(Float) _output_get_2) true true "(R=0.000000,G=1.000000,B=0.095898,A=1.000000)"))
        (:Finished
          (CallFunction|MassInputUn/BLock false)
          (Variables|RoundInfo|SetRound%20State "NewEnumerator3")
          (CallFunction|ResetTimers))))
    (:NewEnumerator3
      (bind _round_time (Timeline|Round%20Timer Play)
        (:Update
          (bind _output_get_3 (Variables|RoundInfo|SetTime _round_time)))
        (:Finished
          (Variables|RoundInfo|SetRound%20Over true)
          (Variables|RoundInfo|SetRound%20State "NewEnumerator4")
          (CallFunction|ResetTimers))))
    (:NewEnumerator4
      (Utilities|FlowControl|DoOnce false :!label _label
        (:Completed
          (bind _output_get_4 (Variables|RoundInfo|Set#%20of%20Rounds (- (Variables|RoundInfo|Get#%20of%20Rounds) 1)))
          (if (not (== _output_get_4 0))
            (CallFunction|CharacterDestroy)
            (Variables|RoundInfo|SetRound%20State "NewEnumerator0")
            (goto _label Reset)))))))

(event Custom|Mass%20Input%20Un/BLock
  (params (Block%20Input? :type Boolean))
  (bind _outactors (Actor|GetAllActorsOfClass "/Game/Flashback_And_Reload/Player/Character_Main.Character_Main_C"))
  (bind _array_element (Utilities|Array|ForEachLoopwithBreak _outactors)
    (:LoopBody
      (Variables|/Game/Flashback_And_Reload/Player/Character_Main.Character_Main_C|SetBlock%20Input _array_element Block%20Input?))))

(event Custom|Spawn%20Characters
  ;[0 0 0] Spawns a player for each connected controller and gives each possession
  (Utilities|FlowControl|Sequence
    (:then_0
      (Utilities|FlowControl|DoOnce false
        (:Completed
          (bind _outactors (Actor|GetAllActorsOfClass "/Game/Flashback_And_Reload/Blueprints/SpawnPoint.SpawnPoint_C"))
          (for _array_element _outactors
            (Utilities|Array|Add (Variables|Default|GetSpawn%20Points) _array_element)))))
    (:then_1
      (bind (_array_element_2 _array_index) (Utilities|Array|ForEachLoopwithBreak (Variables|Default|GetController%20Array))
        (:LoopBody
          (bind (_array_element_3 _array_index_2) (Utilities|Array|ForEachLoopwithBreak (Variables|Default|GetSpawn%20Points) :!label _label)
            (:LoopBody
              (if (== _array_index (Variables|/Game/Flashback_And_Reload/Blueprints/SpawnPoint.SpawnPoint_C|GetPlayer%20Number _array_element_3))
                (bind _returnvalue (Game|SpawnActorfromClass "/Game/Flashback_And_Reload/Player/Character_Main.Character_Main_C" (Variables|/Game/Flashback_And_Reload/Blueprints/SpawnPoint.SpawnPoint_C|GetSpawn%20Transform _array_element_3) true 0 "NewEnumerator0" 0))
                (Pawn|Possess _array_element_2 _returnvalue)
                (Variables|/Game/Flashback_And_Reload/Player/Character_Main.Character_Main_C|SetBlock%20Input _returnvalue true)
                (Utilities|Array|RemoveIndex (Variables|Default|GetSpawn%20Points) _array_index_2)
                (bind _asplayer_state_main (Utilities|Casting|CastToPlayerState_Main (Variables|/Script/Engine.Controller|GetPlayerState _array_element_2))
                  (:then
                    (Utilities|Array|AddUnique (Variables|/Game/Flashback_And_Reload/Player/PlayerState_Main.PlayerState_Main_C|GetCharacter%20References _asplayer_state_main) _returnvalue)
                    (goto _label Break))
                  (:CastFailed
                    (Development|PrintString "Cast to PlayerState_Main in BASIC_GM in Spawn Characters has FAILED")))))))))))

(event Custom|Character%20Destroy
  (bind _outactors (Actor|GetAllActorsOfClass "/Game/Flashback_And_Reload/Player/Character_Main.Character_Main_C"))
  (bind _array_element (Utilities|Array|ForEachLoopwithBreak _outactors)
    (:LoopBody
      (Default|Death _array_element))))

(event EventBeginPlay
  (Utilities|FlowControl|Delay 0.5)
  (CallFunction|StateEvent)
  (Utilities|FlowControl|Gate true) ; enters at Open
)

(event EventPostLogin
  (params (NewPlayer :type Player%20Controller%20Object%20Reference))
  ;[1 1 0] ON LOGIN: Gives Player State a Player ID and adds Player Controller to array
  (Networking|SwitchHasAuthority
    (:Authority
      (bind _asplayer_state_main (Utilities|Casting|CastToPlayerState_Main (Variables|/Script/Engine.Controller|GetPlayerState NewPlayer)))
      (Variables|/Game/Flashback_And_Reload/Player/PlayerState_Main.PlayerState_Main_C|SetPlayer%20Number _asplayer_state_main (- (Utilities|Array|Length (Variables|/Script/Engine.GameState|GetPlayerArray (Game|GetGameState))) 1))
      (bind _asplayer_controller_main (Utilities|Casting|CastToPlayerController_Main NewPlayer)
        (:then
          (Utilities|Array|AddUnique (Variables|Default|GetController%20Array) _asplayer_controller_main))
        (:CastFailed
          (Development|PrintString "PlayerController_Main Cast has failed in Basic_GM"))))))

(event EventTick
  (params (DeltaSeconds :type Float%20%28single-precision%29))
  (Utilities|FlowControl|Gate true
    (:Exit
      (CallFunction|StateEvent))))

(fn ConstructionScript)

(fn ClearAllCharacterArrays
  (bind _array_element (Utilities|Array|ForEachLoopwithBreak (Variables|Default|GetController%20Array))
    (:LoopBody
      (bind _asplayer_state_main (Utilities|Casting|CastToPlayerState_Main (Variables|/Script/Engine.Controller|GetPlayerState _array_element)))
      (Utilities|Array|Clear (Variables|/Game/Flashback_And_Reload/Player/PlayerState_Main.PlayerState_Main_C|GetCharacter%20References _asplayer_state_main)))))