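; Template weapon Blueprint that spawns projectiles ahead of the actor, with automatic or semi-automatic fire, clip and total ammo tracking, and timed reloads.
; FireWeapon and HaultFire drive a set of Gates, with Tick pumping the automatic-fire gate and triggering a reload when the clip empties.
; Automatic shots are spaced by a delay derived from rounds per minute, while semi-automatic shots use an optional pump delay after the first shot.
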(event Custom|Fire%20Weapon
  (Variables|Default|SetFire%20Weapon%20State true)
  (Utilities|FlowControl|Gate false
    (:Exit
      (if (Variables|Type|GetIs%20Weapon%20Automatic?)
        (Utilities|FlowControl|Gate true) ; enters at Open
        (else
          ;[1 1 1] Semiautomatic Weapon Fire
          (if (Variables|State|GetPump%20Delay%20State)
            (Utilities|FlowControl|Delay (Variables|WeaponSpeed|GetPump%20Delay))
            (else
              (Variables|State|SetPump%20Delay%20State true)))
          (CallFunction|FireProjectile)
          (Variables|Ammunition|SetClip%20Ammo (- (Variables|Ammunition|GetClip%20Ammo) 1))
          (Variables|Ammunition|SetCurrent%20Ammo (- (Variables|Ammunition|GetCurrent%20Ammo) 1)))))))

(event Custom|Hault%20Fire
  (Variables|Default|SetFire%20Weapon%20State false)
  (Utilities|FlowControl|Sequence
    (:then_0
      (Utilities|FlowControl|Gate true) ; enters at Open
    )
    (:then_1
      (Utilities|FlowControl|Gate true) ; enters at Close
    )))

(event Custom|Reload%20Weapon
  ;[1 0 0] Reload Weapon
  (Utilities|FlowControl|Sequence
    (:then_0
      (Development|PrintString "Reloading")
      (if (not (== (Variables|Ammunition|GetAmmo%20Capacity%20per%20clip) (Variables|Ammunition|GetClip%20Ammo)))
        (Utilities|FlowControl|Delay (Variables|WeaponSpeed|GetReload%20Speed))
        (Variables|Ammunition|SetClip%20Ammo (Variables|Ammunition|GetAmmo%20Capacity%20per%20clip))
        (if (== (Variables|Ammunition|GetCurrent%20Ammo) 0)
          (Development|PrintString "Out of Ammo" true true "(R=0.073641,G=1.000000,B=0.000000,A=1.000000)")
          (else
            (Utilities|FlowControl|Sequence
              (:then_0
                (Utilities|FlowControl|Gate false) ; enters at Open
              )
              (:then_1
                (if (Variables|Type|GetIs%20Weapon%20Automatic?)
                  (if (Variables|Default|GetFire%20Weapon%20State)
                    (Utilities|FlowControl|Gate true) ; enters at Open
                  ))))))))
    (:then_1
      (Utilities|FlowControl|Gate false) ; enters at Close
    )
    (:then_2
      (Utilities|FlowControl|Gate true) ; enters at Close
    )))

(event EventBeginPlay
  ;[1 1 1] Initialize Ammunition
  (Variables|Ammunition|SetMax%20Ammo (* (Variables|Ammunition|GetClip%20Amount) (Variables|Ammunition|GetAmmo%20Capacity%20per%20clip)))
  (Variables|Ammunition|SetCurrent%20Ammo (Variables|Ammunition|GetMax%20Ammo))
  (Variables|Ammunition|SetClip%20Ammo (Variables|Ammunition|GetAmmo%20Capacity%20per%20clip)))

(event EventTick
  (params (DeltaSeconds :type Float%20%28single-precision%29))
  (if (== (Variables|Ammunition|GetClip%20Ammo) 0)
    (CallFunction|ReloadWeapon))
  (Utilities|FlowControl|Gate true
    (:Exit
      (Utilities|FlowControl|Sequence
        (:then_0
          (Utilities|FlowControl|Gate true :!label _label
            (:Exit
              (CallFunction|FireProjectile)
              (Variables|Ammunition|SetClip%20Ammo (- (Variables|Ammunition|GetClip%20Ammo) 1))
              (Variables|Ammunition|SetCurrent%20Ammo (- (Variables|Ammunition|GetCurrent%20Ammo) 1))
              (goto _label Close))))
        (:then_1
          (bind _delay_between_shots (CallFunction|Rate-of-firetoDelay-between-shots (Variables|WeaponSpeed|GetRate%20of%20Fire)))
          (Utilities|FlowControl|Delay _delay_between_shots)
          (goto _label Open))))))

(fn ConstructionScript)

(fn FireProjectile
  (bind _returnvalue (Transformation|GetActorRotation))
  (Game|SpawnActorfromClass (Variables|Type|GetProjectile) (Math|Transform|MakeTransform (+ (Transformation|GetActorLocation) (* (Math|Vector|GetForwardVector _returnvalue) 1e+02)) _returnvalue "0.500000,0.500000,0.500000") false 0))

(fn Rate-of-firetoDelay-between-shots
  (params (Rate%20of%20Fire :type Float%20%28single-precision%29))
  (return (/ 6e+01 Rate%20of%20Fire)))