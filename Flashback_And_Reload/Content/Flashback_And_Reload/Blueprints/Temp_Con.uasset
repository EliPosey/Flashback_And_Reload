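; Temporary player controller that turns the controlled pawn to face the mouse cursor, forces fullscreen for local players and quits on Escape.
; Each Tick deprojects the cursor to world space and applies only the look-at yaw to the pawn.
; The RInterpTo uses constant delta time and speed whose product exceeds one, so rotation snaps rather than eases.
; AquireMouseLocation stores the cursor's world position but is not called here.
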(event Custom|Aquire%20Mouse%20Location
  (bind (_locationx _locationy) (Game|Player|GetMousePosition))
  (Variables|Default|SetMouse%20Location (.WorldLocation (Class|PlayerController|DeprojectScreenPositiontoWorld _locationx _locationy))))

(event Custom|Rotation
  (bind _returnvalue (Pawn|GetControlledPawn))
  (bind (_locationx _locationy) (Game|Player|GetMousePosition))
  ;[0.07124 1 0] Rotation
  (Transformation|SetActorRotation _returnvalue (Math|Interpolation|RInterpTo (Transformation|GetActorRotation _returnvalue) (Class|KismetMathLibrary|MakeRot 0.0 (.Yaw (Class|KismetMathLibrary|BreakRot (Math|Rotator|FindLookatRotation (Transformation|GetActorLocation _returnvalue) (.WorldLocation (Class|PlayerController|DeprojectScreenPositiontoWorld _locationx _locationy))))) 0.0) 5.0 0.6)))

(event EventTick
  (params (DeltaSeconds :type Float%20%28single-precision%29))
  (CallFunction|Rotation))

(event EventBeginPlay
  ;[1 1 1] Make game Fullscreen Mode
  (if (and (Pawn|IsLocalPlayerController) (not (Networking|IsDedicatedServer)))
    (Development|ExecuteConsoleCommand "FULLSCREEN")))

(event Input|KeyboardEvents|Escape
  (:Pressed
    ;[1 1 1] Quit Game
    (Game|QuitGame 0 "Quit")))

(fn ConstructionScript)